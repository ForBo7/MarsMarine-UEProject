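; Game mode for a Mars marine wave-survival shooter, fading in, looping music and running endless waves of spiders.
; A looping timer spawns each wave's spiders at random TargetPoints, stopping when the quota is spent.
; Registered deaths empty the tracked array, triggering the next wave with a multiplied count and, at set milestones, faster spawns.
; Tick watches for the marine's death to fade out and reload the level; Escape quits.
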(event `Key|Escape`
  (params (Key :type "Key Structure"))
  (:`Pressed`
    (`KismetSystemLibrary.QuitGame` null "Quit")))

(event `End Wave`
  (`KismetSystemLibrary.Delay` 5.0)
  (`self.Start New Wave`))

(event `Spawn Wave`
  (`self.Spawn Spider`))

(event `self.ReceiveBeginPlay`
  (if true
    (`PlayerCameraManager.StartCameraFade` :`self` (`GameplayStatics.GetPlayerCameraManager` 0) :`FromAlpha` 1.0 :`Duration` 4.0)
    (`KismetSystemLibrary.Delay` 2.0)
    (`self.Start New Wave`)
    (bind _returnvalue (`GameplayStatics.SpawnSound2D` "/Game/Sounds/Music/ShooterGame_Music_Cue.ShooterGame_Music_Cue" 1.0 1.0 0.0 null :!label _label))
    (`KismetSystemLibrary.Delay` 10050.0)
    (goto _label)))

(event `self.ReceiveTick`
  (params (DeltaSeconds :type "Float (single-precision)"))
  (bind _asbp_marine (cast `/Game/Blueprints/Pawns/BP_Marine` (`GameplayStatics.GetPlayerCharacter` 0)))
  (if (`/Game/Blueprints/Pawns/BP_Marine.Is Dead` _asbp_marine)
    (`/Engine/EditorBlueprintResources/StandardMacros.DoOnce` false
      (:`Completed`
        (`KismetSystemLibrary.Delay` 2.0)
        (`PlayerCameraManager.StartCameraFade` :`self` (`GameplayStatics.GetPlayerCameraManager` 0) :`ToAlpha` 1.0 :`Duration` 3.0)
        (`AudioComponent.FadeOut` (stale `self.ReceiveBeginPlay` _returnvalue) 2.0 0.0 "Linear")
        (`KismetSystemLibrary.Delay` 2.9)
        (`GameplayStatics.OpenLevel` "Mars")))))

(fn `Get Random Spawn Point`
  (returns (`Spawn Point` :type "TargetPoint Object Reference"))
  (bind _outactors (`GameplayStatics.GetAllActorsOfClass` "/Script/Engine.TargetPoint"))
  (return (`|GetArrayItem` _outactors (`KismetMathLibrary.RandomIntegerInRange` 0 (`KismetArrayLibrary.Array_LastIndex` _outactors)))))

(fn `Increase Wave Difficulty`
  (bind _current_wave (`self.Current Wave`))
  (bind _output_get (set `self.Wave Difficulty` (`KismetMathLibrary.Round` (* (`self.Wave Difficulty`) (`self.Difficulty Multiplier`)))))
  (set `self.Spider Spawns Remaining` _output_get)
  (if (== _current_wave 4)
    (set `self.Duration Between Spawns` 0.8)
    (elif (== _current_wave 7)
      (set `self.Duration Between Spawns` 0.6)
      (elif (== _current_wave 10)
        (set `self.Duration Between Spawns` 0.4)
        (elif (== _current_wave 13)
          (set `self.Duration Between Spawns` 0.2))))))

(fn `Is Wave finished`
  (returns (ReturnValue :type Boolean))
  (return (and (== (`KismetArrayLibrary.Array_Length` (`self.Spiders`)) 0) (== (`self.Spider Spawns Remaining`) 0))))

(fn `Register Spider Death`
  (params (Spider :type "/Game/Blueprints/AI/BP_Great_Spider Object Reference (by ref)"))
  (`KismetArrayLibrary.Array_RemoveItem` (`self.Spiders`) Spider)
  (if (`self.Is Wave finished`)
    (`self.End Wave`)))

(fn `Spawn Spider`
  (bind _spawn_point (`self.Get Random Spawn Point`))
  (`/Engine/EditorBlueprintResources/StandardMacros.IsValid` _spawn_point
    (:`Is Valid`
      (bind _returnvalue (`|SpawnActorFromClass` "/Game/Blueprints/AI/BP_Great_Spider.BP_Great_Spider_C" (`self.GetTransform` _spawn_point) "Undefined" "OverrideRootScale" null null))
      (`/Engine/EditorBlueprintResources/StandardMacros.IsValid` _returnvalue
        (:`Is Valid`
          (`KismetArrayLibrary.Array_Add` (`self.Spiders`) _returnvalue)
          (bind _result (`/Engine/EditorBlueprintResources/StandardMacros.DecrementInt` (`self.Spider Spawns Remaining`))
            (:`  `
              (if (== _result 0)
                (`KismetSystemLibrary.K2_ClearTimer` null "Spawn wave")))))))))

(fn `Start New Wave`
  (`/Engine/EditorBlueprintResources/StandardMacros.IncrementInt` (`self.Current Wave`)
    (:`  `
      (`self.Increase Wave Difficulty`)
      (`KismetSystemLibrary.K2_SetTimer` null "Spawn Wave" (`self.Duration Between Spawns`) true))))

(fn `UserConstructionScript`)
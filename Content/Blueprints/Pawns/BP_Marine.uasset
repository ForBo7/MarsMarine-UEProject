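; BP_Marine is the player marine pawn, with world-axis movement, health, kill count, HUD and death handling.
; Aim sets control yaw from mouse velocity or thumbstick direction, chosen by last key's device, with deadzones and smoothing.
; Firing loops a timed muzzle line trace whose damage grows per hit and resets when firing starts.
; Retriggerable delays force a temporary firing lockout six seconds after the last accepted press or release.
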(event `InputAxis|Move Forward/Backward`
  (params (AxisValue :type "Float (single-precision)"))
  (if (`self.Is Alive`)
    (`self.AddMovementInput` (1.0 0.0 0.0) AxisValue)))

(event `InputAxis|Move Left/Right`
  (params (AxisValue :type "Float (single-precision)"))
  (if (`self.Is Alive`)
    (`self.AddMovementInput` (0.0 1.0 0.0) AxisValue)))

(event `self.ReceiveTick`
  (params (DeltaSeconds :type "Float (single-precision)"))
  (if (`self.Is Alive`)
    (`self.Update Player Aim`)))

(event `Key|AnyKey`
  (params (Key :type "Key Structure"))
  (:`Pressed`
    (set `self.Is Gamepad Key Used` (`KismetInputLibrary.Key_IsGamepadKey` Key))))

(event `InputAction|Fire Weapon`
  (params (Key :type "Key Structure"))
  (:`Pressed`
    (if (`self.Can Shoot`)
      (`self.Start Firing Weapon`)
      (`KismetSystemLibrary.RetriggerableDelay` 6.0 :!label _label)
      (`self.Stop Firing Weapon`)
      (set `self.Can Shoot` false)
      (`KismetSystemLibrary.RetriggerableDelay` 5.0)
      (set `self.Can Shoot` true)))
  (:`Released`
    (`self.Stop Firing Weapon`)
    (if (`self.Can Shoot`)
      (goto _label))))

(event `self.ReceiveBeginPlay`
  (bind _returnvalue (`|CreateWidget` "/Game/UI/W_PlayerHUD.W_PlayerHUD_C" null self))
  (`UserWidget.AddToViewport` _returnvalue 0))

(event `self.ReceiveAnyDamage`
  (params (Damage :type "Float (single-precision)") (DamageType :type "DamageType Object Reference") (InstigatedBy :type "Controller Object Reference") (DamageCauser :type "Actor Object Reference"))
  (bind _new_player_health (`self.Decrease Player Health` Damage))
  (if (== _new_player_health 0.0)
    (set `self.Is Dead` true)
    (`self.Stop Firing Weapon`)
    (`/Engine/EditorBlueprintResources/StandardMacros.DoOnce` false
      (:`Completed`
        (`GameplayStatics.SpawnSound2D` "/Game/Sounds/Stingers/Stereo/Stinger_PlayerDeath_Stereo_Cue.Stinger_PlayerDeath_Stereo_Cue" 1.0 1.0 0.0 null)))))

(fn `Add Health`
  (params (`Health To Add` :type "Float (double-precision)"))
  (set `self.Player Health` (`KismetMathLibrary.FClamp` (+ (`self.Player Health`) `Health To Add`) 0.0 (`self.Max Player Health`))))

(fn `Decrease Player Health`
  (params (`Damage Amount` :type "Float (double-precision)"))
  (returns (`New Player Health` :type "Float (double-precision)"))
  (bind _output_get (set `self.Player Health` (`KismetMathLibrary.FClamp` (- (`self.Player Health`) `Damage Amount`) 0.0 (`self.Max Player Health`))))
  (return _output_get))

(fn `Get Mouse Aim Direction`
  (returns (ReturnValue :type "Rotator Structure"))
  (bind (_returnvalue_x _returnvalue_y) (`KismetMathLibrary.BreakVector2D` (`self.Get Mouse Velocity`)))
  (return (`KismetMathLibrary.RInterpTo` (`Controller.GetControlRotation` (`GameplayStatics.GetPlayerController` 0)) (`KismetMathLibrary.MakeRotator` 0.0 0.0 (`KismetMathLibrary.DegAtan2` _returnvalue_x _returnvalue_y)) (`GameplayStatics.GetWorldDeltaSeconds`) (`self.Mouse Smoothing Strength`))))

(fn `Get Mouse Velocity`
  (returns (ReturnValue :type "Vector2D Structure"))
  (bind (_deltax _deltay) (`PlayerController.GetInputMouseDelta` (`GameplayStatics.GetPlayerController` 0)))
  (return (/ (`KismetMathLibrary.MakeVector2D` _deltax _deltay) (`GameplayStatics.GetWorldDeltaSeconds`))))

(fn `Get Thumbstick Aim Direction`
  (returns (ReturnValue :type "Rotator Structure"))
  (return (`KismetMathLibrary.RInterpTo` (`Controller.GetControlRotation` (`GameplayStatics.GetPlayerController` 0)) (`KismetMathLibrary.MakeRotator` 0.0 0.0 (`KismetMathLibrary.DegAtan2` (`self.GetInputAxisValue`) (`self.GetInputAxisValue`))) (`GameplayStatics.GetWorldDeltaSeconds`) (`self.Thumbstick Smoothing Strength`))))

(fn `Get Weapon Trace End Location`
  (returns (ReturnValue :type "Vector Structure"))
  (return (+ (`self.Get Weapon Trace Start Location`) (* (`KismetMathLibrary.GetForwardVector` (`self.GetControlRotation`)) (`self.Weapon Range`)))))

(fn `Get Weapon Trace Start Location`
  (returns (ReturnValue :type "Vector Structure"))
  (return (`SceneComponent.GetSocketLocation` (`self.Rifle`) "MuzzleFlashSocket")))

(fn `Increase Player Kills`
  (`/Engine/EditorBlueprintResources/StandardMacros.IncrementInt` (`self.Player Kills`)))

(fn `Is Alive`
  (returns (ReturnValue :type Boolean))
  (return (not (`self.Is Dead`))))

(fn `Is Health Full`
  (returns (ReturnValue :type Boolean))
  (return (== (`self.Player Health`) (`self.Max Player Health`))))

(fn `Is Mouse Above Deadzone`
  (returns (ReturnValue :type Boolean))
  (return (> (`KismetMathLibrary.VSize2D` (`self.Get Mouse Velocity`)) (`self.Mouse Deadzone`))))

(fn `Is Thumbstick Above Deadzone`
  (returns (ReturnValue :type Boolean))
  (return (> (`KismetMathLibrary.VSize2D` (`KismetMathLibrary.MakeVector2D` (`self.GetInputAxisValue`) (`self.GetInputAxisValue`))) (`self.Thumbstick Deadzone`))))

(fn `Set Can Shoot To True`)

(fn `Spawn Impact Hit`
  (params (`Spawn Location` :type "Vector Structure"))
  (`GameplayStatics.SpawnEmitterAtLocation` "/Game/Effects/Weapons/Impacts/P_AssaultRifle_IH.P_AssaultRifle_IH" `Spawn Location`))

(fn `Start Firing Weapon`
  (if (`self.Is Alive`)
    (set `self.Damage Per Shot` 10.0)
    (`ActorComponent.Activate` (`self.P_AssaultRifle_MF`) false)
    (`GameplayStatics.SpawnSound2D` "/Game/Sounds/Weapon_AssaultRifle/Stereo/RifleFireStart_Cue.RifleFireStart_Cue" 1.0 1.0 0.0 null)
    (bind _returnvalue (`GameplayStatics.SpawnSound2D` "/Game/Sounds/Weapon_AssaultRifle/Stereo/RifleFireLoop_Cue.RifleFireLoop_Cue" 1.0 1.0 0.0 null))
    (set `self.Rifle Fire Sound` _returnvalue)
    (`self.Weapon Trace`)
    (`KismetSystemLibrary.K2_SetTimer` null "Weapon Trace" (`self.Fire Rate`) true)))

(fn `Stop Firing Weapon`
  (`ActorComponent.Deactivate` (`self.P_AssaultRifle_MF`))
  (`AudioComponent.Stop` (`self.Rifle Fire Sound`))
  (`KismetSystemLibrary.K2_ClearTimer` null "Weapon Trace")
  (if (`self.Is Alive`)
    (`GameplayStatics.SpawnSound2D` "/Game/Sounds/Weapon_AssaultRifle/Stereo/RiflelFireEnd_Cue.RiflelFireEnd_Cue" 1.0 1.0 0.0 null) ; Delete this if things get too buggy
  ))

(fn `Update Mouse Aim`
  (if (`self.Is Mouse Above Deadzone`)
    (`Controller.SetControlRotation` (`GameplayStatics.GetPlayerController` 0) (`self.Get Mouse Aim Direction`))))

(fn `Update Player Aim`
  (if (`self.Is Gamepad Key Used`)
    (`self.Update Thumbstick Aim`)
    (else
      (`self.Update Mouse Aim`))))

(fn `Update Thumbstick Aim`
  (if (`self.Is Thumbstick Above Deadzone`)
    (`Controller.SetControlRotation` (`GameplayStatics.GetPlayerController` 0) (`self.Get Thumbstick Aim Direction`))))

(fn `UserConstructionScript`)

(fn `Weapon Trace`
  (bind (_outhit _returnvalue) (`KismetSystemLibrary.LineTraceSingle` (`self.Get Weapon Trace Start Location`) (`self.Get Weapon Trace End Location`) "TraceTypeQuery1"))
  (if _returnvalue
    (bind (_bblockinghit _binitialoverlap _time _distance _location _impactpoint _normal _impactnormal _physmat _hitactor) (`GameplayStatics.BreakHitResult` _outhit))
    (`GameplayStatics.ApplyDamage` _hitactor (`self.Damage Per Shot`))
    (`self.Spawn Impact Hit` _location)
    (set `self.Damage Per Shot` (+ (`self.Damage Per Shot`) 0.5))))